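; BP_Window is the card target frame of a Struck Out game, where actors tagged "Ball" knock out cards.
; Each card's box overlap spawns BP_CardGC in its place, hides the card and disables that box's collision.
; Regular cards increment CardCounter on StruckOutGameInstance, while the skull card (Card4) sets GameOverFlag.
; Two item cards lower KickCounter by subtraction clamped at zero or by halving; an unconnected increase branch never runs.
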(event OnComponentBeginOverlap(Box)
  (params (OverlappedComponent :type Primitive%20Component%20Object%20Reference) (OtherActor :type Actor%20Object%20Reference) (OtherComp :type Primitive%20Component%20Object%20Reference) (OtherBodyIndex :type Integer) (bFromSweep :type Boolean) (SweepResult :type Hit%20Result%20Structure%20%28by%20ref%29))
  (bind _card_5 (Variables|Default|GetCard_5))
  (if (Actor|ActorHasTag OtherActor "Ball")
    (Game|SpawnActorfromClass "/Game/Card/Card_GC/BP_CardGC.BP_CardGC_C" (Math|Transform|MakeTransform (Transformation|GetWorldLocation _card_5) (Transformation|GetWorldRotation _card_5) "1.000000,1.000000,1.000000") "Undefined" "MultiplyWithRoot" 0 0)
    (Rendering|SetVisibility (Variables|Default|GetCard_5) false false)
    (Collision|SetCollisionEnabled (Variables|Default|GetBox) "NoCollision")
    (CallFunction|CardCounterIncFunc)))

(event OnComponentBeginOverlap(Box7)
  (params (OverlappedComponent :type Primitive%20Component%20Object%20Reference) (OtherActor :type Actor%20Object%20Reference) (OtherComp :type Primitive%20Component%20Object%20Reference) (OtherBodyIndex :type Integer) (bFromSweep :type Boolean) (SweepResult :type Hit%20Result%20Structure%20%28by%20ref%29))
  (bind _card_7 (Variables|Default|GetCard_7))
  (if (Actor|ActorHasTag OtherActor "Ball")
    (Game|SpawnActorfromClass "/Game/Card/Card_GC/BP_CardGC.BP_CardGC_C" (Math|Transform|MakeTransform (Transformation|GetWorldLocation _card_7) (Transformation|GetWorldRotation _card_7) "1.000000,1.000000,1.000000") "Undefined" "MultiplyWithRoot" 0 0)
    (Rendering|SetVisibility (Variables|Default|GetCard_7) false false)
    (Collision|SetCollisionEnabled (Variables|Default|GetBox7) "NoCollision")
    (CallFunction|CardCounterIncFunc)))

(event OnComponentBeginOverlap(Box_8)
  (params (OverlappedComponent :type Primitive%20Component%20Object%20Reference) (OtherActor :type Actor%20Object%20Reference) (OtherComp :type Primitive%20Component%20Object%20Reference) (OtherBodyIndex :type Integer) (bFromSweep :type Boolean) (SweepResult :type Hit%20Result%20Structure%20%28by%20ref%29))
  (bind _card_8 (Variables|Default|GetCard_8))
  (if (Actor|ActorHasTag OtherActor "Ball")
    (Game|SpawnActorfromClass "/Game/Card/Card_GC/BP_CardGC.BP_CardGC_C" (Math|Transform|MakeTransform (Transformation|GetWorldLocation _card_8) (Transformation|GetWorldRotation _card_8) "1.000000,1.000000,1.000000") "Undefined" "MultiplyWithRoot" 0 0)
    (Rendering|SetVisibility (Variables|Default|GetCard_8) false false)
    (Collision|SetCollisionEnabled (Variables|Default|GetBox_8) "NoCollision")
    (CallFunction|CardCounterIncFunc)))

(event OnComponentBeginOverlap(Box_9)
  (params (OverlappedComponent :type Primitive%20Component%20Object%20Reference) (OtherActor :type Actor%20Object%20Reference) (OtherComp :type Primitive%20Component%20Object%20Reference) (OtherBodyIndex :type Integer) (bFromSweep :type Boolean) (SweepResult :type Hit%20Result%20Structure%20%28by%20ref%29))
  (bind _card_9 (Variables|Default|GetCard_9))
  (if (Actor|ActorHasTag OtherActor "Ball")
    (Game|SpawnActorfromClass "/Game/Card/Card_GC/BP_CardGC.BP_CardGC_C" (Math|Transform|MakeTransform (Transformation|GetWorldLocation _card_9) (Transformation|GetWorldRotation _card_9) "1.000000,1.000000,1.000000") "Undefined" "MultiplyWithRoot" 0 0)
    (Rendering|SetVisibility (Variables|Default|GetCard_9) false false)
    (Collision|SetCollisionEnabled (Variables|Default|GetBox_9) "NoCollision")
    (CallFunction|CardCounterIncFunc)))

(event OnComponentBeginOverlap(box10)
  (params (OverlappedComponent :type Primitive%20Component%20Object%20Reference) (OtherActor :type Actor%20Object%20Reference) (OtherComp :type Primitive%20Component%20Object%20Reference) (OtherBodyIndex :type Integer) (bFromSweep :type Boolean) (SweepResult :type Hit%20Result%20Structure%20%28by%20ref%29))
  (bind _card_10 (Variables|Default|GetCard_10))
  (if (Actor|ActorHasTag OtherActor "Ball")
    (Game|SpawnActorfromClass "/Game/Card/Card_GC/BP_CardGC.BP_CardGC_C" (Math|Transform|MakeTransform (Transformation|GetWorldLocation _card_10) (Transformation|GetWorldRotation _card_10) "1.000000,1.000000,1.000000") "Undefined" "MultiplyWithRoot" 0 0)
    (Rendering|SetVisibility (Variables|Default|GetCard_10) false false)
    (Collision|SetCollisionEnabled (Variables|Default|Getbox10) "NoCollision")
    (CallFunction|CardCounterIncFunc)))

(event OnComponentBeginOverlap(Box_3)
  (params (OverlappedComponent :type Primitive%20Component%20Object%20Reference) (OtherActor :type Actor%20Object%20Reference) (OtherComp :type Primitive%20Component%20Object%20Reference) (OtherBodyIndex :type Integer) (bFromSweep :type Boolean) (SweepResult :type Hit%20Result%20Structure%20%28by%20ref%29))
  (bind _card_3 (Variables|Default|GetCard_3))
  (if (Actor|ActorHasTag OtherActor "Ball")
    (Game|SpawnActorfromClass "/Game/Card/Card_GC/BP_CardGC.BP_CardGC_C" (Math|Transform|MakeTransform (Transformation|GetWorldLocation _card_3) (Transformation|GetWorldRotation _card_3) "1.000000,1.000000,1.000000") "Undefined" "MultiplyWithRoot" 0 0)
    (Rendering|SetVisibility (Variables|Default|GetCard_3) false false)
    (Collision|SetCollisionEnabled (Variables|Default|GetBox_3) "NoCollision")
    (CallFunction|CardCounterIncFunc)))

(event OnComponentBeginOverlap(Box_1)
  (params (OverlappedComponent :type Primitive%20Component%20Object%20Reference) (OtherActor :type Actor%20Object%20Reference) (OtherComp :type Primitive%20Component%20Object%20Reference) (OtherBodyIndex :type Integer) (bFromSweep :type Boolean) (SweepResult :type Hit%20Result%20Structure%20%28by%20ref%29))
  (bind _card_1 (Variables|Default|GetCard_1))
  (if (Actor|ActorHasTag OtherActor "Ball")
    (Game|SpawnActorfromClass "/Game/Card/Card_GC/BP_CardGC.BP_CardGC_C" (Math|Transform|MakeTransform (Transformation|GetWorldLocation _card_1) (Transformation|GetWorldRotation _card_1) "1.000000,1.000000,1.000000") "Undefined" "MultiplyWithRoot" 0 0)
    (Rendering|SetVisibility (Variables|Default|GetCard_1) false false)
    (Collision|SetCollisionEnabled (Variables|Default|GetBox_1) "NoCollision")
    (CallFunction|CardCounterIncFunc)))

(event OnComponentBeginOverlap(Box_2)
  (params (OverlappedComponent :type Primitive%20Component%20Object%20Reference) (OtherActor :type Actor%20Object%20Reference) (OtherComp :type Primitive%20Component%20Object%20Reference) (OtherBodyIndex :type Integer) (bFromSweep :type Boolean) (SweepResult :type Hit%20Result%20Structure%20%28by%20ref%29))
  (bind _card_2 (Variables|Default|GetCard_2))
  (if (Actor|ActorHasTag OtherActor "Ball")
    (Game|SpawnActorfromClass "/Game/Card/Card_GC/BP_CardGC.BP_CardGC_C" (Math|Transform|MakeTransform (Transformation|GetWorldLocation _card_2) (Transformation|GetWorldRotation _card_2) "1.000000,1.000000,1.000000") "Undefined" "MultiplyWithRoot" 0 0)
    (Rendering|SetVisibility (Variables|Default|GetCard_2) false false)
    (Collision|SetCollisionEnabled (Variables|Default|GetBox_2) "NoCollision")
    (CallFunction|CardCounterIncFunc)))

(event OnComponentBeginOverlap(Box_4)
  (params (OverlappedComponent :type Primitive%20Component%20Object%20Reference) (OtherActor :type Actor%20Object%20Reference) (OtherComp :type Primitive%20Component%20Object%20Reference) (OtherBodyIndex :type Integer) (bFromSweep :type Boolean) (SweepResult :type Hit%20Result%20Structure%20%28by%20ref%29))
  (bind _card_4 (Variables|Default|GetCard_4))
  ;[0.15 0.15 0.15 0.5] Special Cards
  ;;[0.15 0.15 0.15 0.5] skull card
  (if (Actor|ActorHasTag OtherActor "Ball")
    (Game|SpawnActorfromClass "/Game/Card/Card_GC/BP_CardGC.BP_CardGC_C" (Math|Transform|MakeTransform (Transformation|GetWorldLocation _card_4) (Transformation|GetWorldRotation _card_4) "1.000000,1.000000,1.000000") "Undefined" "MultiplyWithRoot" 0 0)
    (Rendering|SetVisibility (Variables|Default|GetCard_4) false false)
    (Collision|SetCollisionEnabled (Variables|Default|GetBox_4) "NoCollision")
    (bind _asstruck_out_game_instance (Utilities|Casting|CastToStruckOutGameInstance (Game|GetGameInstance)))
    (Variables|/Game/ThirdPerson/Maps/StruckOutGameInstance.StruckOutGameInstance_C|SetGameOverFlag _asstruck_out_game_instance true)))

(event OnComponentBeginOverlap(Box_6)
  (params (OverlappedComponent :type Primitive%20Component%20Object%20Reference) (OtherActor :type Actor%20Object%20Reference) (OtherComp :type Primitive%20Component%20Object%20Reference) (OtherBodyIndex :type Integer) (bFromSweep :type Boolean) (SweepResult :type Hit%20Result%20Structure%20%28by%20ref%29))
  (bind _card_6 (Variables|Default|GetCard_6))
  (if (Actor|ActorHasTag OtherActor "Ball")
    (Game|SpawnActorfromClass "/Game/Card/Card_GC/BP_CardGC.BP_CardGC_C" (Math|Transform|MakeTransform (Transformation|GetWorldLocation _card_6) (Transformation|GetWorldRotation _card_6) "1.000000,1.000000,1.000000") "Undefined" "MultiplyWithRoot" 0 0)
    (Rendering|SetVisibility (Variables|Default|GetCard_6) false false)
    (Collision|SetCollisionEnabled (Variables|Default|GetBox_6) "NoCollision")
    (CallFunction|CardCounterIncFunc)))

(event OnComponentBeginOverlap(Box_Item2)
  (params (OverlappedComponent :type Primitive%20Component%20Object%20Reference) (OtherActor :type Actor%20Object%20Reference) (OtherComp :type Primitive%20Component%20Object%20Reference) (OtherBodyIndex :type Integer) (bFromSweep :type Boolean) (SweepResult :type Hit%20Result%20Structure%20%28by%20ref%29))
  (bind _card_item_2 (Variables|Default|GetCard_Item_2))
  ;[0.15 0.15 0.15 0.5] Special Cards
  (if (Actor|ActorHasTag OtherActor "Ball")
    (Game|SpawnActorfromClass "/Game/Card/Card_GC/BP_CardGC.BP_CardGC_C" (Math|Transform|MakeTransform (Transformation|GetWorldLocation _card_item_2) (Transformation|GetWorldRotation _card_item_2) "1.000000,1.000000,1.000000") "Undefined" "MultiplyWithRoot" 0 0)
    (Rendering|SetVisibility (Variables|Default|GetCard_Item_2) false false)
    (Collision|SetCollisionEnabled (Variables|Default|GetBox_Item2) "NoCollision")
    (bind _asstruck_out_game_instance (Utilities|Casting|CastToStruckOutGameInstance (Game|GetGameInstance)))
    ;;[0.15 0.15 0.15 0.5] Comment
    (Variables|/Game/ThirdPerson/Maps/StruckOutGameInstance.StruckOutGameInstance_C|SetKickCounter _asstruck_out_game_instance (/ (Variables|/Game/ThirdPerson/Maps/StruckOutGameInstance.StruckOutGameInstance_C|GetKickCounter _asstruck_out_game_instance) 2))))

(event OnComponentBeginOverlap(Box_Item1)
  (params (OverlappedComponent :type Primitive%20Component%20Object%20Reference) (OtherActor :type Actor%20Object%20Reference) (OtherComp :type Primitive%20Component%20Object%20Reference) (OtherBodyIndex :type Integer) (bFromSweep :type Boolean) (SweepResult :type Hit%20Result%20Structure%20%28by%20ref%29))
  (bind _card_item_1 (Variables|Default|GetCard_Item_1))
  ;[0.15 0.15 0.15 0.5] Special Cards
  (if (Actor|ActorHasTag OtherActor "Ball")
    (Game|SpawnActorfromClass "/Game/Card/Card_GC/BP_CardGC.BP_CardGC_C" (Math|Transform|MakeTransform (Transformation|GetWorldLocation _card_item_1) (Transformation|GetWorldRotation _card_item_1) "1.000000,1.000000,1.000000") "Undefined" "MultiplyWithRoot" 0 0)
    (Rendering|SetVisibility (Variables|Default|GetCard_Item_1) false false)
    (Collision|SetCollisionEnabled (Variables|Default|GetBox_Item1) "NoCollision")
    (bind _asstruck_out_game_instance (Utilities|Casting|CastToStruckOutGameInstance (Game|GetGameInstance)))
    (if (< (- (Variables|/Game/ThirdPerson/Maps/StruckOutGameInstance.StruckOutGameInstance_C|GetKickCounter _asstruck_out_game_instance) 3) 0)
      (Variables|/Game/ThirdPerson/Maps/StruckOutGameInstance.StruckOutGameInstance_C|SetKickCounter _asstruck_out_game_instance 0)
      (else
        (Variables|/Game/ThirdPerson/Maps/StruckOutGameInstance.StruckOutGameInstance_C|SetKickCounter _asstruck_out_game_instance (- (Variables|/Game/ThirdPerson/Maps/StruckOutGameInstance.StruckOutGameInstance_C|GetKickCounter _asstruck_out_game_instance) 3))))))

(event EventBeginPlay)

(event Collision|EventActorBeginOverlap
  (params (OtherActor :type Actor%20Object%20Reference)))

(event EventTick
  (params (DeltaSeconds :type Float%20%28single-precision%29)))

(fn ConstructionScript)

(fn CardCounterIncFunc
  (bind _asstruck_out_game_instance (Utilities|Casting|CastToStruckOutGameInstance (Game|GetGameInstance)))
  (Math|Integer|IncrementInt (Variables|/Game/ThirdPerson/Maps/StruckOutGameInstance.StruckOutGameInstance_C|GetCardCounter _asstruck_out_game_instance)))