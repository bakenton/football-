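; Kickable ball that, on first contact with the player character's foot capsule, increments the game instance's kick counter and is replaced by a kicked-ball actor.
; The character's KickST value selects a spawn function for the high, low or mid ball variant.
; Each spawns at the ball's location along the player's arrow rotation, adding random upward pitch.
; The original ball then hides, disables its sphere collision and destroys itself after a delay.
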(event OnComponentBeginOverlap(Sphere)
  (params (OverlappedComponent :type Primitive%20Component%20Object%20Reference) (OtherActor :type Actor%20Object%20Reference) (OtherComp :type Primitive%20Component%20Object%20Reference) (OtherBodyIndex :type Integer) (bFromSweep :type Boolean) (SweepResult :type Hit%20Result%20Structure%20%28by%20ref%29))
  (bind _asbp_third_person_character (Utilities|Casting|CastToBP_ThirdPersonCharacter OtherActor))
  (bind _ascapsule_collision (Utilities|Casting|CastToCapsuleComponent OtherComp))
  (if (== _ascapsule_collision (Variables|/Game/ThirdPerson/Blueprints/BP_ThirdPersonCharacter.BP_ThirdPersonCharacter_C|GetFoot_Capsule _asbp_third_person_character))
    (Utilities|FlowControl|DoOnce false
      (:Completed
        (bind _asstruck_out_game_instance (Utilities|Casting|CastToStruckOutGameInstance (Game|GetGameInstance)))
        (Math|Integer|IncrementInt (Variables|/Game/ThirdPerson/Maps/StruckOutGameInstance.StruckOutGameInstance_C|GetKickCounter _asstruck_out_game_instance)
          (:%20%20
            (switch int (Variables|/Game/ThirdPerson/Blueprints/BP_ThirdPersonCharacter.BP_ThirdPersonCharacter_C|GetKick_ST _asbp_third_person_character)
              (:0
                (CallFunction|BallHiSpawnFunc))
              (:1
                (CallFunction|BallLowSpawnFunc))
              (:2
                (CallFunction|BallMidSpawnFunc)))
            (Rendering|SetVisibility (Variables|Default|Getball) false false)
            (Collision|SetCollisionEnabled (Variables|Default|GetSphere) "NoCollision")
            (Utilities|FlowControl|Delay 4.0)
            (Actor|DestroyActor)))))))

(event EventBeginPlay)

(event Collision|EventActorBeginOverlap
  (params (OtherActor :type Actor%20Object%20Reference)))

(event EventTick
  (params (DeltaSeconds :type Float%20%28single-precision%29)))

(fn ConstructionScript)

(fn BallHiSpawnFunc
  (bind _asbp_third_person_character (Utilities|Casting|CastToBP_ThirdPersonCharacter (Game|Player|GetPlayerPawn 0)))
  (Game|SpawnActorfromClass "/Game/Ball/BP_Ball_Hi.BP_Ball_Hi_C" (Math|Transform|MakeTransform (Transformation|GetWorldLocation (Variables|Default|Getball)) (Math|Rotator|MakeRotator (.roll (Transformation|GetWorldRotation (Variables|/Game/ThirdPerson/Blueprints/BP_ThirdPersonCharacter.BP_ThirdPersonCharacter_C|GetPlayer_Arrow _asbp_third_person_character))) (+ (.pitch (Transformation|GetWorldRotation (Variables|/Game/ThirdPerson/Blueprints/BP_ThirdPersonCharacter.BP_ThirdPersonCharacter_C|GetPlayer_Arrow _asbp_third_person_character))) (Math|Random|RandomFloatinRange 2e+01 5e+01)) (.yaw (Transformation|GetWorldRotation (Variables|/Game/ThirdPerson/Blueprints/BP_ThirdPersonCharacter.BP_ThirdPersonCharacter_C|GetPlayer_Arrow _asbp_third_person_character)))) "1.000000,1.000000,1.000000") "Undefined" "MultiplyWithRoot" 0 0))

(fn BallMidSpawnFunc
  (bind _asbp_third_person_character (Utilities|Casting|CastToBP_ThirdPersonCharacter (Game|Player|GetPlayerPawn 0)))
  (Game|SpawnActorfromClass "/Game/Ball/BP_Ball_Mid.BP_Ball_Mid_C" (Math|Transform|MakeTransform (Transformation|GetWorldLocation (Variables|Default|Getball)) (Math|Rotator|MakeRotator (.roll (Transformation|GetWorldRotation (Variables|/Game/ThirdPerson/Blueprints/BP_ThirdPersonCharacter.BP_ThirdPersonCharacter_C|GetPlayer_Arrow _asbp_third_person_character))) (+ (.pitch (Transformation|GetWorldRotation (Variables|/Game/ThirdPerson/Blueprints/BP_ThirdPersonCharacter.BP_ThirdPersonCharacter_C|GetPlayer_Arrow _asbp_third_person_character))) (Math|Random|RandomFloatinRange 15.0 25.0)) (.yaw (Transformation|GetWorldRotation (Variables|/Game/ThirdPerson/Blueprints/BP_ThirdPersonCharacter.BP_ThirdPersonCharacter_C|GetPlayer_Arrow _asbp_third_person_character)))) "1.000000,1.000000,1.000000") "Undefined" "MultiplyWithRoot" 0 0))

(fn BallLowSpawnFunc
  (bind _asbp_third_person_character (Utilities|Casting|CastToBP_ThirdPersonCharacter (Game|Player|GetPlayerPawn 0)))
  (Game|SpawnActorfromClass "/Game/Ball/BP_Ball_Low.BP_Ball_Low_C" (Math|Transform|MakeTransform (Transformation|GetWorldLocation (Variables|Default|Getball)) (Math|Rotator|MakeRotator (.roll (Transformation|GetWorldRotation (Variables|/Game/ThirdPerson/Blueprints/BP_ThirdPersonCharacter.BP_ThirdPersonCharacter_C|GetPlayer_Arrow _asbp_third_person_character))) (+ (.pitch (Transformation|GetWorldRotation (Variables|/Game/ThirdPerson/Blueprints/BP_ThirdPersonCharacter.BP_ThirdPersonCharacter_C|GetPlayer_Arrow _asbp_third_person_character))) (Math|Random|RandomFloatinRange 2e+01 3e+01)) (+ (.yaw (Transformation|GetWorldRotation (Variables|/Game/ThirdPerson/Blueprints/BP_ThirdPersonCharacter.BP_ThirdPersonCharacter_C|GetPlayer_Arrow _asbp_third_person_character))) 0.0)) "1.000000,1.000000,1.000000") "Undefined" "MultiplyWithRoot" 0 0))